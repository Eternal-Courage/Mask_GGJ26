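; BP_MaskPickup is a mask collectible that grants the first-person character an ability on overlap, then destroys itself.
; MaskType selects the mesh in the construction script and the DT_Masks row cached at BeginPlay, which the pickup never reads.
; Overlap directly boosts walk speed, enables trash collection or boosts jump and air control for three mask types.
; Mask UI, collection and ability-reset logic is disconnected.
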(event `self.ReceiveBeginPlay`
  ;[0 0 0] Get Row with all data for New Mask
  (bind _returnvalue (`|GetDataTableRow` "/Game/Taylor/Misc/DT_Masks.DT_Masks" (`|GetEnumeratorName` (`self. Mask Type`)))
    (:`then`
      (set `self.Mask Row Data` _returnvalue))))

(event `self.Collider.OnComponentBeginOverlap`
  (params (OverlappedComponent :type "PrimitiveComponent Object Reference") (OtherActor :type "Actor Object Reference") (OtherComp :type "PrimitiveComponent Object Reference") (OtherBodyIndex :type Integer) (bFromSweep :type Boolean) (SweepResult :type "HitResult Structure (by ref)"))
  (bind _charactermovement (`Character.CharacterMovement` (`self.As BP First Person Character`)))
  (bind _charactermovement_2 (`Character.CharacterMovement` (`self.As BP First Person Character`)))
  (bind _charactermovement_3 (`Character.CharacterMovement` (`self.As BP First Person Character`)))
  (bind _asbp_first_person_character (cast `/Game/FirstPerson/Blueprints/BP_FirstPersonCharacter` OtherActor))
  (set `self.As BP First Person Character` _asbp_first_person_character)
  (`self.K2_DestroyActor`)
  (switch `/Game/Taylor/Misc/E_MaskType` (`self. Mask Type`)
    (:`NewEnumerator0`
      ;[0 0 0] Movement Speed
      (set `CharacterMovementComponent.MaxWalkSpeed` (* (`CharacterMovementComponent.MaxWalkSpeed` _charactermovement_2) 1.5) _charactermovement_2))
    (:`NewEnumerator6`
      ;[0 0 0] Collect Trash
      (set `/Game/FirstPerson/Blueprints/BP_FirstPersonCharacter.CanCollectTrash?` true (`self.As BP First Person Character`)))
    (:`NewEnumerator7`
      ;[0 0 0] Jump Height
      (set `CharacterMovementComponent.JumpZVelocity` (* (`CharacterMovementComponent.JumpZVelocity` _charactermovement_3) 1.5) _charactermovement)
      (set `CharacterMovementComponent.AirControl` (* (`CharacterMovementComponent.AirControl` _charactermovement) 1.5) _charactermovement_3))))

(fn `UserConstructionScript`
  (`StaticMeshComponent.SetStaticMesh` (`self.MaskMesh`) (select `/Game/Taylor/Misc/E_MaskType` (`self. Mask Type`) :`NewEnumerator0` "/Game/Taylor/MaskMeshes/Running_mask.Running_mask" :`NewEnumerator4` "/Game/Taylor/MaskMeshes/Climbing_Mask.Climbing_Mask" :`NewEnumerator5` "/Game/Taylor/MaskMeshes/Trash_Mask.Trash_Mask" :`NewEnumerator6` "/Game/Taylor/MaskMeshes/Jumping_mask.Jumping_mask" :`NewEnumerator7` "/Game/Taylor/MaskMeshes/Ending_Mask.Ending_Mask" :!type "StaticMesh Object Reference")))