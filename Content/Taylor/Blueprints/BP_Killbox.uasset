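; BP_Killbox is a kill volume that destroys the player and triggers a respawn when a BP_FirstPersonCharacter overlaps it.
; On overlap, a Sequence first casts and stores BP_FirstPersonGameMode, then disables input, destroys the character and calls the game mode's RespawnPlayer.
; The kill step always targets player index 0 rather than the overlapping actor.
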(event `self.ReceiveActorBeginOverlap`
  (params (OtherActor :type "Actor Object Reference"))
  (cast `/Game/FirstPerson/Blueprints/BP_FirstPersonCharacter` OtherActor)
  (`|ExecutionSequence`
    (:`then_0`
      (bind _asbp_first_person_game_mode (cast `/Game/FirstPerson/Blueprints/BP_FirstPersonGameMode` (`GameplayStatics.GetGameMode`)))
      (set `self.Game Mode` _asbp_first_person_game_mode))
    (:`then_1`
      ;[0 0 0] Kill Player
      (`self.DisableInput` (`GameplayStatics.GetPlayerController` 0))
      (`self.K2_DestroyActor` (`GameplayStatics.GetPlayerCharacter` 0))
      (`/Game/FirstPerson/Blueprints/BP_FirstPersonGameMode.Respawn Player` (`self.Game Mode`)))))

(fn `UserConstructionScript`)