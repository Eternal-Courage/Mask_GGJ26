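; BP_TrashItem is a trash pickup that the first-person character can collect with the interact action.
; Overlapping its collider shows the character's HUD button prompt and binds PickUpItem to the character's OnInteract event; leaving hides and unbinds it.
; PickUpItem simply destroys the actor.
; The construction script sets the mesh from the TrashType value, either cigarette or soda bottle.
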(event `self.Collider.OnComponentBeginOverlap`
  (params (OverlappedComponent :type "PrimitiveComponent Object Reference") (OtherActor :type "Actor Object Reference") (OtherComp :type "PrimitiveComponent Object Reference") (OtherBodyIndex :type Integer) (bFromSweep :type Boolean) (SweepResult :type "HitResult Structure (by ref)"))
  (bind _asbp_first_person_character (cast `/Game/FirstPerson/Blueprints/BP_FirstPersonCharacter` OtherActor))
  (bind _output_get (set `self.As BP First Person Character` _asbp_first_person_character))
  (`Widget.SetVisibility` (`/Game/Taylor/Blueprints/UI/WBP_HUD.ButtonPrompt` (`/Game/FirstPerson/Blueprints/BP_FirstPersonCharacter.HUD` _output_get)) "Visible")
  (add `/Game/FirstPerson/Blueprints/BP_FirstPersonCharacter.OnInteract` _output_get (delegate `Pick Up Item`)))

(event `Pick Up Item`
  (`self.K2_DestroyActor`))

(event `self.Collider.OnComponentEndOverlap`
  (params (OverlappedComponent :type "PrimitiveComponent Object Reference") (OtherActor :type "Actor Object Reference") (OtherComp :type "PrimitiveComponent Object Reference") (OtherBodyIndex :type Integer))
  (bind _asbp_first_person_character (cast `/Game/FirstPerson/Blueprints/BP_FirstPersonCharacter` OtherActor))
  (`Widget.SetVisibility` (`/Game/Taylor/Blueprints/UI/WBP_HUD.ButtonPrompt` (`/Game/FirstPerson/Blueprints/BP_FirstPersonCharacter.HUD` _asbp_first_person_character)) "Collapsed")
  (remove `/Game/FirstPerson/Blueprints/BP_FirstPersonCharacter.OnInteract` _asbp_first_person_character (delegate `Pick Up Item`)))

(fn `UserConstructionScript`
  (`StaticMeshComponent.SetStaticMesh` (`self.Trash Mesh`) (select `/Game/Taylor/Misc/TrashType` (`self.TrashType`) :`NewEnumerator0` "/Game/Brae_Assets/Assets_programmer_friendly/Smoke.Smoke" :`NewEnumerator1` "/Game/Kaylee/Assets/Brae/Server.Server" :!type "StaticMesh Object Reference")))