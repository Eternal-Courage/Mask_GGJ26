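; BP_Ladder is a ladder actor meant to let the player climb by pressing E.
; Collider begin overlap shows a prompt widget; end overlap, behind a validity check, removes it, stops climbing, disables input and resets a DoOnce.
; E fires that DoOnce to start climbing on PlayerCharacter.
; The graph looks unfinished: casts lack target classes, PlayerCharacter is set to None, and EnableInput is disconnected.
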(event `self.Collider.OnComponentBeginOverlap`
  (params (OverlappedComponent :type "PrimitiveComponent Object Reference") (OtherActor :type "Actor Object Reference") (OtherComp :type "PrimitiveComponent Object Reference") (OtherBodyIndex :type Integer) (bFromSweep :type Boolean) (SweepResult :type "HitResult Structure (by ref)"))
  (bind _asbp_third_person_character_tunnel (cast `` OtherActor))
  (set `self.PlayerCharacter` null _asbp_third_person_character_tunnel)
  (bind _returnvalue (`|CreateWidget` null null "Press E to use ladder"))
  (`UserWidget.AddToViewport` _returnvalue 0))

(event `self.Collider.OnComponentEndOverlap`
  (params (OverlappedComponent :type "PrimitiveComponent Object Reference") (OtherActor :type "Actor Object Reference") (OtherComp :type "PrimitiveComponent Object Reference") (OtherBodyIndex :type Integer))
  (bind (_playercharacter _playercharacter_2) (`self.PlayerCharacter`))
  (bind _asbp_third_person_character_tunnel (cast `` OtherActor))
  (`/Engine/EditorBlueprintResources/StandardMacros.IsValid` null
    (:`Is Valid`
      (`Widget.RemoveFromParent` null)
      (`self.StopClimbing` _asbp_third_person_character_tunnel)
      (`self.DisableInput` (`GameplayStatics.GetPlayerController` 0))
      (goto _label :!via `Reset`))))

(event `Key|E`
  (params (Key :type "Key Structure"))
  (bind (_playercharacter _playercharacter_2) (`self.PlayerCharacter`))
  (:`Pressed`
    (`/Engine/EditorBlueprintResources/StandardMacros.DoOnce` false :!label _label
      (:`Completed`
        (`/Engine/EditorBlueprintResources/StandardMacros.IsValid` _playercharacter_2
          (:`Is Valid`
            (`self.StartClimbing` _playercharacter_2)))))))

(fn `UserConstructionScript`)